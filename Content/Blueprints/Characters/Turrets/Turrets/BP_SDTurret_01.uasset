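; BP_SDTurret_01 is a turret character Blueprint that supplies turret-specific data to the systems that query it.
; It overrides getters to return its current target, its actor type gameplay tag and AM_Turret_01_Fire as the shooting montage.
; The hit react montage getter returns nothing, and the construction script only calls its parent, so the file defines no targeting or firing logic of its own.
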(fn ConstructionScript
  (|CallParentFunction))

(fn TurretGetCurrentTarget0
  (return (Variables|Default|GetCurrentTarget)))

(fn GetActorTypeGameplayTag
  (return (Variables|Default|GetActorTypeTag)))

(fn GetHitReactMontage
  (return 0))

(fn GetShootingMontage
  (return "/Game/Assets/Turret/Animations/AM_Turret_01_Fire.AM_Turret_01_Fire"))