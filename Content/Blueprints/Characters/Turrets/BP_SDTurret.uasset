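; BP_SDTurret is a turret that sequences waking, aiming and shooting at a target, with timed delays between stages.
; The server caches the Blackboard, while clients disable actor tick on BeginPlay.
; Combat start waits out an awakening timer, then enables aiming and tick if the target is valid.
; Targeting requires shooting gameplay tags, rechecking them after a delay before calling HandleShooting.
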(event EventBeginPlay
  (|CallParentFunction)
  (if (Networking|IsServer)
    (Variables|Default|SetBlackboard (AI|GetBlackboard 0))
    (else
      (Actor|Tick|SetActorTickEnabled false)))
  (Variables|Default|SetStartingLocation (- (.location (Transformation|GetWorldTransform (Variables|Character|GetMesh))) (Variables|Default|GetTargetOffsetVector))))

(event Collision|EventActorBeginOverlap
  (params (OtherActor :type Actor%20Object%20Reference))
  (|CallParentFunction OtherActor) ; This node is disabled and will not be called.\nDrag off pins to build functionality.
)

(event EventStartCombatState
  (Utilities|FlowControl|Delay (Variables|Default|GetTurretAfterAwakeningTimer))
  (Utilities|IsValid (Variables|Default|GetCurrentTarget)
    (:Is%20Valid
      (Variables|Default|SetbIsAiming true)
      (Actor|Tick|SetActorTickEnabled true))))

(event EventStartTargeting
  (if (Class|SDCharacterBase|HasGameplayTag (Variables|Default|GetTurretShootingTags))
    (Variables|Default|SetbIsTargetting true)
    (Utilities|FlowControl|Delay (Variables|Default|GetTurretAfterTargetingTimer))
    (if (Class|SDCharacterBase|HasGameplayTag (Variables|Default|GetTurretShootingTags))
      (Class|SDTurret|HandleShooting))))

(fn ConstructionScript)

(fn GetActorTypeGameplayTag
  (return (Variables|Default|GetActorTypeTag)))