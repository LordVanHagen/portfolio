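; Gameplay ability that fires a predicted projectile for turret combat actors; other actor types have no firing logic here.
; An AI target-trace task on the turret's current target supplies target data, then the actor's shooting montage plays.
; Montage gameplay events time the shot, spawning the projectile from the trace hit, and later end the ability.
; A failed trace or an interrupted or cancelled montage also ends it.
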(event Ability|EventActivateAbility
  (bind _ascombat_interface (Utilities|Casting|CastToCombatInterface (Ability|GetAvatarActorfromActorInfo)))
  (bind _returnvalue (Class|CombatInterface|GetShootingMontage _ascombat_interface))
  (Variables|Default|SetShootingMontage _returnvalue)
  (if (== (Class|CombatInterface|GetActorTypeGameplayTag _ascombat_interface) "(TagName=\"Combat.Actor.Turret\")")
    (bind _datahandle (|AITargetTrace (Class|CombatInterface|TurretGetCurrentTarget _ascombat_interface) false)
      (:ValidData
        (|PlayMontageandWaitProxy "None" (Variables|Default|GetShootingMontage) 1.0 "None" true 1.0 0.0 false
          (:then
            (Ability|Tasks|WaitGameplayEvent "(TagName=\"Event.Montage.Shoot\")" 0
              (:EventReceived
                (Class|SDShootPredictedProjectile|SpawnPredictedProjectile (Ability|TargetData|GetHitResultfromTargetData _datahandle))
                (Ability|Tasks|WaitGameplayEvent "(TagName=\"Event.Montage.Finished\")" 0
                  (:EventReceived
                    (Ability|EndAbility))))))
          (:OnInterrupted
            (Ability|EndAbility :!label _label))
          (:OnCancelled
            (goto _label))))
      (:OnFailed
        (Ability|EndAbility)))))

(event Ability|EventOnEndAbility
  (params (bWasCancelled :type Boolean)))